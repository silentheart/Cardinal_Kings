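; GodlyLightning is a lightning strike hazard actor that damages the player standing inside its T7 zone.
; Overlap events on T7 track whether MyCharacter is in range and store a reference to it.
; The Strike event shows lightning flipbooks on seven sprites, then clears them and disarms after a short delay.
; While armed, Tick calls the player's DamageSystem once and plays a thunder sound, then disarms.
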(event OnComponentBeginOverlap(T7)
  (params (OtherActor :type Actor%20Object%20Reference) (OtherComp :type Primitive%20Component%20Object%20Reference) (OtherBodyIndex :type Integer) (bFromSweep :type Boolean) (SweepResult :type Hit%20Result%20Structure%20%28by%20ref%29))
  ;[1 1 1] Lightning Zones
  (bind _asmy_character (Utilities|Casting|CastToMyCharacter OtherActor))
  (Variables|Default|SetInRangeSeven true)
  (Variables|Default|SetPlayerRef _asmy_character))

(event OnComponentEndOverlap(T7)
  (params (OtherActor :type Actor%20Object%20Reference) (OtherComp :type Primitive%20Component%20Object%20Reference) (OtherBodyIndex :type Integer))
  ;[1 1 1] Lightning Zones
  (Utilities|Casting|CastToMyCharacter OtherActor)
  (Variables|Default|SetInRangeSeven false))

(event Custom|Strike
  ;[1 1 1] Strike
  (Variables|Default|SetIsSeven true)
  (Utilities|FlowControl|Sequence
    (:then_0
      (Sprite|SetFlipbook (Variables|Default|GetI1M) "/Game/Game/Flipbook/lightning.lightning"))
    (:then_1
      (Sprite|SetFlipbook (Variables|Default|GetI3-R) "/Game/Game/Flipbook/lightning.lightning")
      (Sprite|SetFlipbook (Variables|Default|GetI3-L) "/Game/Game/Flipbook/lightning.lightning"))
    (:then_2
      (Sprite|SetFlipbook (Variables|Default|GetI5-R) "/Game/Game/Flipbook/lightning.lightning")
      (Sprite|SetFlipbook (Variables|Default|GetI5-L) "/Game/Game/Flipbook/lightning.lightning"))
    (:then_3
      (Sprite|SetFlipbook (Variables|Default|GetI7-R) "/Game/Game/Flipbook/lightning.lightning")
      (Sprite|SetFlipbook (Variables|Default|GetI7-L) "/Game/Game/Flipbook/lightning.lightning"))
    (:then_4
      (Utilities|FlowControl|Delay 0.8)
      (Utilities|FlowControl|Sequence
        (:then_0
          (Sprite|SetFlipbook (Variables|Default|GetI1M)))
        (:then_1
          (Sprite|SetFlipbook (Variables|Default|GetI3-R))
          (Sprite|SetFlipbook (Variables|Default|GetI3-L)))
        (:then_2
          (Sprite|SetFlipbook (Variables|Default|GetI5-R))
          (Sprite|SetFlipbook (Variables|Default|GetI5-L)))
        (:then_3
          (Sprite|SetFlipbook (Variables|Default|GetI7-R))
          (Sprite|SetFlipbook (Variables|Default|GetI7-L)))
        (:then_4
          (Variables|Default|SetIsSeven false))))))

(event EventBeginPlay
  ;[1 1 1] Strike
  (Utilities|FlowControl|Sequence
    (:then_0
      (Sprite|SetFlipbook (Variables|Default|GetI1M)))
    (:then_1
      (Sprite|SetFlipbook (Variables|Default|GetI3-R))
      (Sprite|SetFlipbook (Variables|Default|GetI3-L)))
    (:then_2
      (Sprite|SetFlipbook (Variables|Default|GetI5-R))
      (Sprite|SetFlipbook (Variables|Default|GetI5-L)))
    (:then_3
      (Sprite|SetFlipbook (Variables|Default|GetI7-R))
      (Sprite|SetFlipbook (Variables|Default|GetI7-L)))
    (:then_4
      (Variables|Default|SetIsSeven false))))

(event EventTick
  (params (DeltaSeconds :type Float%20%28single-precision%29))
  ;[1 1 1] DealDamage
  (if (and (Variables|Default|GetIsSeven) (Variables|Default|GetInRangeSeven))
    (Default|DamageSystem (Variables|Default|GetPlayerRef) (Variables|Default|GetPlayerDamage))
    (Audio|SpawnSoundatLocation "/Game/Sounds/Thunder_02.Thunder_02" (Transformation|GetActorLocation))
    (Variables|Default|SetIsSeven false)))

(fn ConstructionScript)