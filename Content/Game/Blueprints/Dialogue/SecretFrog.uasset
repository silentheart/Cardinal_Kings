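; SecretFrog is a dialogue actor that speaks to the player and teleports them to a hard-coded location, apparently a secret area.
; It creates a dialogue widget on BeginPlay, and box overlap by the player runs DialogueMacro to scroll speech text into it.
; An index check leads to a short delay before the teleport.
; Leaving the box removes the widget and resets the talking state and index.
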(event OnComponentEndOverlap(Box)
  (params (OtherActor :type Actor%20Object%20Reference) (OtherComp :type Primitive%20Component%20Object%20Reference) (OtherBodyIndex :type Integer))
  (Widget|RemovefromParent (Variables|Default|GetWidget))
  (Variables|Default|SetIsTalking false)
  (Variables|Default|SetIndex 0))

(event OnComponentBeginOverlap(Box)
  (params (OtherActor :type Actor%20Object%20Reference) (OtherComp :type Primitive%20Component%20Object%20Reference) (OtherBodyIndex :type Integer) (bFromSweep :type Boolean) (SweepResult :type Hit%20Result%20Structure%20%28by%20ref%29))
  (bind _widget (Variables|Default|GetWidget))
  (if (== OtherActor (Game|GetPlayerCharacter 0))
    (for _index (range 0 0)
      (Utilities|DialogueMacro (Variables|Default|GetTestingStringArray) (Variables|Default|GetAppendStringTo) (Variables|Default|GetArrayChar) (Variables|Default|GetIndex) 0.05 0.0 (Variables|/Game/Game/Blueprints/Dialogue/Dialogue_Widget.Dialogue_Widget_C|GetDialogue_String _widget) _widget (Variables|Default|GetIsTalking))
      (if (< (Variables|Default|GetIndex) 3)
        (Variables|Default|SetIndex (+ (Variables|Default|GetIndex) 1))
        (Utilities|FlowControl|Delay 1.0)
        (bind _asmy_character (Utilities|Casting|CastToMyCharacter OtherActor))
        (Transformation|Teleport _asmy_character "-24809.066406, 0,572.372559" "0, 0, 0")
        (else
          (Variables|Default|SetIndex 0))))
    (Variables|Default|SetIndex 0)))

(event EventBeginPlay)

(event Collision|EventActorBeginOverlap
  (params (OtherActor :type Actor%20Object%20Reference)))

(event EventTick
  (params (DeltaSeconds :type Float%20%28single-precision%29)))

(event EventBeginPlay
  (Utilities|Casting|CastToMyCharacter (Game|GetPlayerCharacter 0))
  (bind _returnvalue (UserInterface|CreateWidget "/Game/Game/Blueprints/Dialogue/Dialogue_Widget.Dialogue_Widget_C"))
  (Variables|Default|SetWidget _returnvalue)
  (Variables|Default|SetPlayerController 0))

(fn ConstructionScript)