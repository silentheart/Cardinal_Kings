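; BP_Bull is a bullet-like actor that kills enemies it overlaps and destroys itself 15 seconds after spawning.
; Actor overlap runs a cast chain over Frog, Bird, Frog2, Sheepie and Lotus, calling KillFrog on a match and playing a sound, without destroying itself.
; It is also destroyed when a Float_Enemy_damage actor leaves its BulletRange component.
; Older DamageEnemy and Enemy_BP logic remains unconnected.
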(event OnComponentBeginOverlap(BulletRange)
  (params (OtherActor :type Actor%20Object%20Reference) (OtherComp :type Primitive%20Component%20Object%20Reference) (OtherBodyIndex :type Integer) (bFromSweep :type Boolean) (SweepResult :type Hit%20Result%20Structure%20%28by%20ref%29)))

(event OnComponentEndOverlap(BulletRange)
  (params (OtherActor :type Actor%20Object%20Reference) (OtherComp :type Primitive%20Component%20Object%20Reference) (OtherBodyIndex :type Integer))
  (Utilities|Casting|CastToFloat_Enemy_damage OtherActor)
  (Actor|DestroyActor))

(event EventBeginPlay
  (Utilities|FlowControl|Delay 15.0)
  (Actor|DestroyActor))

(event EventTick
  (params (DeltaSeconds :type Float%20%28single-precision%29)))

(event Collision|EventActorBeginOverlap
  (params (OtherActor :type Actor%20Object%20Reference))
  ;[1 1 1] Kill Enemies
  (Utilities|FlowControl|Sequence
    (:then_0
      (bind _asfrog (Utilities|Casting|CastToFrog OtherActor))
      (Default|KillFrog _asfrog)
      (Audio|PlaySoundatLocation "/Game/Sounds/Frog_Vox.Frog_Vox" (Transformation|GetActorLocation)))
    (:then_1
      (bind _asbird (Utilities|Casting|CastToBird OtherActor))
      (Default|KillFrog _asbird)
      (Audio|PlaySoundatLocation "/Game/Sounds/Bird_Flap.Bird_Flap" (Transformation|GetActorLocation)))
    (:then_2
      (bind _asfrog_2 (Utilities|Casting|CastToFrog2 OtherActor))
      (Default|KillFrog _asfrog_2)
      (Audio|PlaySoundatLocation "/Game/Sounds/Frog_Vox.Frog_Vox" (Transformation|GetActorLocation)))
    (:then_3
      (bind _assheepie (Utilities|Casting|CastToSheepie OtherActor))
      (Default|KillFrog _assheepie)
      (Audio|SpawnSoundatLocation "/Game/Sounds/Blossom_Warning.Blossom_Warning" (Transformation|GetActorLocation)))
    (:then_4
      (bind _aslotus (Utilities|Casting|CastToLotus OtherActor))
      (Default|KillFrog _aslotus)
      (Audio|SpawnSoundatLocation "/Game/Sounds/Blossom_Latch.Blossom_Latch" (Transformation|GetActorLocation)))))

(fn ConstructionScript)