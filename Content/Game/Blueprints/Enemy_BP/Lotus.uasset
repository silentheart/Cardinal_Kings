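; Lotus enemy Blueprint, apparently adapted from a frog enemy, that acts as a touch hazard for the player.
; Overlapping its TouchBox passes DamageVal to the player's DamageSystem unless IsDead is set.
; KillFrog and BeginPlay do nothing, and Tick loops over all BP_Bull actors without acting on them.
; Death flipbook, left/right patrol, bullet range check and health-loss logic remain as disconnected nodes that never run.
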(event OnComponentBeginOverlap(TouchBox)
  (params (OtherActor :type Actor%20Object%20Reference) (OtherComp :type Primitive%20Component%20Object%20Reference) (OtherBodyIndex :type Integer) (bFromSweep :type Boolean) (SweepResult :type Hit%20Result%20Structure%20%28by%20ref%29))
  ;[1 1 1] Damage
  ;;[1 1 1] Damage By Touch
  (if (and (not (Variables|Default|GetIsDead)) (== OtherActor (Game|GetPlayerCharacter 0)))
    (bind _asmy_character (Utilities|Casting|CastToMyCharacter OtherActor))
    (Default|DamageSystem _asmy_character (Variables|Default|GetDamage%20Val))))

(event Custom|KillFrog
  ;[1 1 1] Frog Death
  (if (not (Variables|Default|GetIsDead))
    _))

(event EventTick
  (params (DeltaSeconds :type Float%20%28single-precision%29))
  ;[1 1 1] Event Tick
  (if (not (Variables|Default|GetIsDead))
    (Utilities|FlowControl|Sequence
      (:then_1
        (bind _outactors (Actor|GetAllActorsOfClass "/Game/Game/Blueprints/BP_Bull.BP_Bull_C"))
        (for _array_element _outactors
          _)))))

(event EventBeginPlay
  ;[1 1 1] Begin Play
)

(fn ConstructionScript)