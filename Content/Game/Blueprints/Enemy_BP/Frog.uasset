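; Frog enemy for a Paper2D game that spits BP_Frog_Shot projectiles and damages the player on touch through MyCharacter's DamageSystem.
; BulletRange overlaps set IsSpotted, which Tick reads to fire from Arrow1, with delays timing the attack flipbook and cooldown.
; KillFrog plays the death flipbook, disables capsule collision, removes movement, then destroys the actor after a delay.
; Patrol and proximity-damage logic is disconnected, and the per-tick BP_Bull search does nothing.
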(event OnComponentBeginOverlap(BulletRange)
  (params (OtherActor :type Actor%20Object%20Reference) (OtherComp :type Primitive%20Component%20Object%20Reference) (OtherBodyIndex :type Integer) (bFromSweep :type Boolean) (SweepResult :type Hit%20Result%20Structure%20%28by%20ref%29))
  ;[1 1 1] Damage
  ;;[1 1 1] Damage Range
  (Variables|Default|SetIsSpotted (== OtherActor (Game|GetPlayerCharacter 0))))

(event OnComponentEndOverlap(BulletRange)
  (params (OtherActor :type Actor%20Object%20Reference) (OtherComp :type Primitive%20Component%20Object%20Reference) (OtherBodyIndex :type Integer))
  ;[1 1 1] Damage
  ;;[1 1 1] Damage Range
  (Variables|Default|SetIsSpotted (not (== OtherActor (Game|GetPlayerCharacter 0)))))

(event OnComponentBeginOverlap(TouchBox)
  (params (OtherActor :type Actor%20Object%20Reference) (OtherComp :type Primitive%20Component%20Object%20Reference) (OtherBodyIndex :type Integer) (bFromSweep :type Boolean) (SweepResult :type Hit%20Result%20Structure%20%28by%20ref%29))
  ;[1 1 1] Damage
  ;;[1 1 1] Damage By Touch
  (if (and (not (Variables|Default|GetIsDead)) (== OtherActor (Game|GetPlayerCharacter 0)))
    (bind _asmy_character (Utilities|Casting|CastToMyCharacter OtherActor))
    (Default|DamageSystem _asmy_character (Variables|Default|GetDamage%20Val))))

(event Custom|KillFrog
  ;[1 1 1] Frog Death
  (if (not (Variables|Default|GetIsDead))
    (Sprite|SetFlipbook (Variables|Default|GetPaperFlipbook) "/Game/Game/Sprites/Enemies/Frog/FrogDeath/EnemyFrog_Death.EnemyFrog_Death")
    (Variables|Default|SetIsDead true)
    (Collision|SetCollisionEnabled (Variables|Collision|GetCapsuleComponent) "NoCollision")
    (Components|DestroyComponent (Variables|Character|GetCharacterMovement))
    (Utilities|FlowControl|Delay 1.5)
    (Actor|DestroyActor)))

(event EventTick
  (params (DeltaSeconds :type Float%20%28single-precision%29))
  ;[1 1 1] Event Tick
  (if (not (Variables|Default|GetIsDead))
    (Utilities|FlowControl|Sequence
      (:then_1
        (bind _outactors (Actor|GetAllActorsOfClass "/Game/Game/Blueprints/BP_Bull.BP_Bull_C"))
        (for _array_element _outactors
          _))
      (:then_2
        ;[1 1 1] Damage
        ;;[1 1 1] Damage By Range
        (if (and (not (Variables|Default|GetIsDead)) (and (Variables|Default|GetIsSpotted) (not (Variables|Default|GetHasShot))))
          (Game|SpawnActorfromClass "/Game/Game/Blueprints/BP_Frog_Shot.BP_Frog_Shot_C" (Transformation|GetWorldTransform (Variables|Default|GetArrow1)) "Undefined" 0 0)
          (Audio|SpawnSoundatLocation "/Game/Sounds/Frog_Spit.Frog_Spit" (Transformation|GetActorLocation))
          (Variables|Default|SetHasShot true)
          (Sprite|SetFlipbook (Variables|Default|GetPaperFlipbook) "/Game/Game/Sprites/Enemies/Frog/FrogAttack/EnemyFrog_Attack.EnemyFrog_Attack")
          (Utilities|FlowControl|Delay 0.5)
          (Sprite|SetFlipbook (Variables|Default|GetPaperFlipbook) "/Game/Game/Sprites/Enemies/Frog/FrogIdle/EnemyFrog_Idle.EnemyFrog_Idle")
          (Utilities|FlowControl|Delay 1.5)
          (Variables|Default|SetHasShot false))))))

(event EventBeginPlay
  ;[1 1 1] Begin Play
)

(fn ConstructionScript)