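; Pickup item that fully restores the player character's health and chi when walked into.
; On box overlap with the player character, a sequence first raises CurrentHealth to MaxHealth, plays a low-pitched Whip_Attack sound at the item's location and destroys the actor.
; The sequence's second branch then raises ChiLevel to MaxChi, after the destroy call.
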(event OnComponentBeginOverlap(Box)
  (params (OtherActor :type Actor%20Object%20Reference) (OtherComp :type Primitive%20Component%20Object%20Reference) (OtherBodyIndex :type Integer) (bFromSweep :type Boolean) (SweepResult :type Hit%20Result%20Structure%20%28by%20ref%29))
  (bind _returnvalue (Game|GetPlayerCharacter 0))
  (if (== OtherActor _returnvalue)
    (Utilities|FlowControl|Sequence
      (:then_0
        (bind _asmy_character (Utilities|Casting|CastToMyCharacter _returnvalue))
        (Variables|/Game/Game/Blueprints/MyCharacter.MyCharacter_C|SetCurrentHealth _asmy_character (+ (Variables|/Game/Game/Blueprints/MyCharacter.MyCharacter_C|GetCurrentHealth _asmy_character) (- (Variables|/Game/Game/Blueprints/MyCharacter.MyCharacter_C|GetMaxHealth _asmy_character) (Variables|/Game/Game/Blueprints/MyCharacter.MyCharacter_C|GetCurrentHealth _asmy_character))))
        (Audio|SpawnSoundatLocation "/Game/Sounds/Whip_Attack.Whip_Attack" (Transformation|GetActorLocation) "0, 0, 0" 1.0 0.2)
        (Actor|DestroyActor))
      (:then_1
        (bind _asmy_character_2 (Utilities|Casting|CastToMyCharacter _returnvalue))
        (Variables|/Game/Game/Blueprints/MyCharacter.MyCharacter_C|SetChiLevel _asmy_character_2 (+ (Variables|/Game/Game/Blueprints/MyCharacter.MyCharacter_C|GetChiLevel _asmy_character_2) (- (Variables|/Game/Game/Blueprints/MyCharacter.MyCharacter_C|GetMaxChi _asmy_character_2) (Variables|/Game/Game/Blueprints/MyCharacter.MyCharacter_C|GetChiLevel _asmy_character_2))))))))

(event EventBeginPlay)

(event Collision|EventActorBeginOverlap
  (params (OtherActor :type Actor%20Object%20Reference)))

(event EventTick
  (params (DeltaSeconds :type Float%20%28single-precision%29)))

(fn ConstructionScript)