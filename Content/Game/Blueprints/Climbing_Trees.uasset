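; Climbable tree actor that uses two box triggers to toggle climbing on MyCharacter.
; Entering Box sets CanClimb and clears PlayerTouching, while entering Box1 clears CanClimb after a short delay.
; Leaving Box1 sets PlayerTouching, and a delayed Box1 entry with that flag set adds a new box component at runtime.
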(event OnComponentBeginOverlap(Box1)
  (params (OtherActor :type Actor%20Object%20Reference) (OtherComp :type Primitive%20Component%20Object%20Reference) (OtherBodyIndex :type Integer) (bFromSweep :type Boolean) (SweepResult :type Hit%20Result%20Structure%20%28by%20ref%29))
  (bind _asmy_character (Utilities|Casting|CastToMyCharacter OtherActor))
  (Utilities|FlowControl|Delay 0.2)
  (Variables|/Game/Game/Blueprints/MyCharacter.MyCharacter_C|SetCanClimb _asmy_character false)
  (if (Variables|Default|GetPlayerTouching?)
    (AddComponent|AddBoxComponent false)))

(event OnComponentEndOverlap(Box1)
  (params (OtherActor :type Actor%20Object%20Reference) (OtherComp :type Primitive%20Component%20Object%20Reference) (OtherBodyIndex :type Integer))
  (Utilities|Casting|CastToMyCharacter OtherActor)
  (Variables|Default|SetPlayerTouching? true))

(event OnComponentBeginOverlap(Box)
  (params (OtherActor :type Actor%20Object%20Reference) (OtherComp :type Primitive%20Component%20Object%20Reference) (OtherBodyIndex :type Integer) (bFromSweep :type Boolean) (SweepResult :type Hit%20Result%20Structure%20%28by%20ref%29))
  (bind _asmy_character (Utilities|Casting|CastToMyCharacter OtherActor))
  (Variables|/Game/Game/Blueprints/MyCharacter.MyCharacter_C|SetCanClimb _asmy_character true)
  (Variables|Default|SetPlayerTouching? false))

(event EventBeginPlay)

(event EventActorBeginOverlap
  (params (OtherActor :type Actor%20Object%20Reference)))

(event EventTick
  (params (DeltaSeconds :type Float%20%28single-precision%29)))

(fn ConstructionScript)