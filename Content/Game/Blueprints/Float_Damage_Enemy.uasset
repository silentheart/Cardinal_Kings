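; Enemy actor that patrols back and forth along X from its spawn location and damages MyCharacter when it overlaps its Box.
; Tick flips a Left flag at X thresholds to drive MoveComponentTo and rotation, and prints the location each frame.
; DamageEnemy subtracts fixed health, destroys the actor at zero or below, and spawns an animated floating widget showing remaining health after a short delay.
; An unconnected target-point patrol loop never runs.
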(event OnComponentBeginOverlap(Box)
  (params (OtherActor :type Actor%20Object%20Reference) (OtherComp :type Primitive%20Component%20Object%20Reference) (OtherBodyIndex :type Integer) (bFromSweep :type Boolean) (SweepResult :type Hit%20Result%20Structure%20%28by%20ref%29))
  (bind _asmy_character (Utilities|Casting|CastToMyCharacter OtherActor))
  (Default|DamageSystem _asmy_character (Variables|Default|GetDamage%20Val)))

(event Custom|DamageEnemy
  ;[1 1 1] Deals damage to the enemy.
  (Utilities|FlowControl|Sequence
    (:then_0
      (bind _returnvalue (UserInterface|CreateWidget "/Game/Game/Blueprints/FloatingText_Widget.FloatingText_Widget_C" 0 self))
      (Utilities|FlowControl|Delay 0.2)
      (Variables|/Game/Game/Blueprints/FloatingText_Widget.FloatingText_Widget_C|SetFloat%20Damage _returnvalue (Math|Conversions|ToFloat(Integer) (Variables|Default|GetEnemy%20Health)))
      (UserInterface|Viewport|AddtoViewport _returnvalue 0)
      (UserInterface|Animation|PlayAnimation _returnvalue (Variables|/Game/Game/Blueprints/FloatingText_Widget.FloatingText_Widget_C|GetFloating%20Text%20ani _returnvalue) 0.0 1 "Forward"))
    (:then_1
      (bind _output_get (Variables|Default|SetEnemy%20Health (- (Variables|Default|GetEnemy%20Health) 34)))
      (if (<= _output_get 0)
        (Actor|DestroyActor)))))

(event EventBeginPlay
  (Variables|Default|SetTargetLocation (Transformation|GetActorLocation)))

(event EventTick
  (params (DeltaSeconds :type Float%20%28single-precision%29))
  (bind _returnvalue (VehicleSound|GetRootComponent))
  (bind _returnvalue_2 (Transformation|GetActorLocation))
  (bind _targetlocation (Variables|Default|GetTargetLocation))
  (bind _x (Math|Vector|BreakVector _targetlocation))
  (bind _x_2 (Math|Vector|BreakVector _returnvalue_2))
  (Utilities|FlowControl|Sequence
    (:then_0
      (if (Variables|Default|GetLeft)
        (Transformation|SetRelativeRotation _returnvalue "0.000000, 0, 0" false false)
        (Components|MoveComponentTo _returnvalue (- _targetlocation "1000.000000, 0, 0") "0, 0, 0" false false 2.0)
        (else
          (Transformation|SetRelativeRotation _returnvalue "0.000000,180.000000, 0" false false)
          (Components|MoveComponentTo _returnvalue _targetlocation "0.000000, 0,0.000000" false false 2.0))))
    (:then_1
      (if (>= _x_2 (- _x 5e+01))
        (Variables|Default|SetLeft true)))
    (:then_2
      (if (<= _x_2 (- _x 5e+02))
        (Variables|Default|SetLeft false)))
    (:then_3
      (Development|PrintString (Utilities|String|ToString(Vector) _returnvalue_2)))))

(event Collision|EventActorBeginOverlap
  (params (OtherActor :type Actor%20Object%20Reference)))

(fn ConstructionScript)