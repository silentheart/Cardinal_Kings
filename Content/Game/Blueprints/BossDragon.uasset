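; BossDragon is a Paper2D boss that loses health when BP_Bull actors hit its box, destroying them.
; Tick splits health into four bar segments, overwriting Health with Health/MaxHealth each pass, and reveals the widget after an entrance delay.
; Tick also rolls randomly for a roar-and-lightning attack; a roots variant is unwired.
; At zero health it plays a death sound, disables input, then pauses and shows EndGame.
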(event OnComponentBeginOverlap(Box)
  (params (OtherActor :type Actor%20Object%20Reference) (OtherComp :type Primitive%20Component%20Object%20Reference) (OtherBodyIndex :type Integer) (bFromSweep :type Boolean) (SweepResult :type Hit%20Result%20Structure%20%28by%20ref%29))
  ;[1 1 1] DamageSystem
  (bind _asbp_bull (Utilities|Casting|CastToBP_Bull OtherActor))
  (Actor|DestroyActor _asbp_bull)
  (Variables|Default|SetHealth (- (Variables|Default|GetHealth) (Variables|Default|GetDmgTaken))))

(event Custom|Update%20Health%20Percent
  (bind _maxhealth (Variables|Default|GetMaxHealth))
  (bind _maxhealth_2 (Variables|Default|GetMaxHealth))
  (bind _maxhealth_3 (Variables|Default|GetMaxHealth))
  ;[1 1 1] Health Percent Update
  (Variables|Default|SetHealth%25 (/ (Variables|Default|GetHealth) (Variables|Default|GetMaxHealth)))
  (if (> (Variables|Default|GetHealth%25) 0.75)
    (Variables|Default|SetH4%25 (/ (- (Variables|Default|GetHealth) (* _maxhealth 0.75)) (/ _maxhealth 4.0)))
    (Variables|Default|SetH3%25 1.0)
    (Variables|Default|SetH2%25 1.0)
    (Variables|Default|SetH1%25 1.0)
    (elif (> (Variables|Default|GetHealth%25) 0.5)
      (Variables|Default|SetH4%25 0.0)
      (Variables|Default|SetH3%25 (/ (- (Variables|Default|GetHealth) (* _maxhealth_2 0.5)) (/ _maxhealth_2 4.0)))
      (Variables|Default|SetH2%25 1.0)
      (Variables|Default|SetH1%25 1.0)
      (elif (> (Variables|Default|GetHealth%25) 0.25)
        (Variables|Default|SetH4%25 0.0)
        (Variables|Default|SetH3%25 0.0)
        (Variables|Default|SetH2%25 (/ (- (Variables|Default|GetHealth) (* _maxhealth_3 0.25)) (/ _maxhealth_3 4.0)))
        (Variables|Default|SetH1%25 1.0)
        (elif (> (Variables|Default|GetHealth%25) 0.0)
          (Variables|Default|SetH4%25 0.0)
          (Variables|Default|SetH3%25 0.0)
          (Variables|Default|SetH2%25 0.0)
          (Variables|Default|SetH1%25 (/ (Variables|Default|GetHealth) (/ (Variables|Default|GetMaxHealth) 4.0)))
          (else
            (Variables|Default|SetIsDead true)
            (Variables|Default|SetH1%25 0.0)
            (Audio|SpawnSoundatLocation "/Game/Sounds/Dragon_Death.Dragon_Death" (Transformation|GetActorLocation))
            (Input|DisableInput (Game|GetPlayerController 0))
            (Utilities|FlowControl|Delay 5.0)
            (Game|SetGamePaused true)
            (bind _returnvalue (UserInterface|CreateWidget "/Game/Game/Widgets/EndGame.EndGame_C"))
            (UserInterface|Viewport|AddtoViewport _returnvalue 0)
            (Variables|/Script/Engine.PlayerController|SetbShowMouseCursor (Game|GetPlayerController 0) true)))))))

(event EventBeginPlay
  ;[1 1 1] BeginPlay
  (bind _returnvalue (UserInterface|CreateWidget "/Game/Game/Blueprints/BossHealthBar.BossHealthBar_C"))
  (bind _output_get (Variables|Default|SetHealthBar _returnvalue)))

(event EventTick
  (params (DeltaSeconds :type Float%20%28single-precision%29))
  ;[1 1 1] LRA Fire Check
  (if (not (Variables|Default|GetIsDead))
    (Utilities|FlowControl|Sequence
      (:then_0
        (CallFunction|UpdateHealthPercent))
      (:then_1
        (CallFunction|UpdateHealth))
      (:then_2
        (if (>= (Math|Random|RandomFloatinRange (Variables|Default|GetLRA_Min) (Variables|Default|GetLRA_Max)) (Variables|Default|GetLRA_Req))
          (Sprite|SetFlipbook (Variables|Default|GetPaperFlipbook) "/Game/Game/Sprites/Enemies/Dragon/Dragon_RangedAtt.Dragon_RangedAtt")
          (Audio|SpawnSoundatLocation "/Game/Sounds/Dragon_Roar.Dragon_Roar" (Transformation|GetActorLocation))
          (Utilities|FlowControl|Delay 0.4)
          (Default|Strike (Variables|Default|GetLightningRef))
          (Utilities|FlowControl|Delay 0.4)
          (Sprite|SetFlipbook (Variables|Default|GetPaperFlipbook) "/Game/Game/Sprites/Enemies/Dragon/Dragon_Idle.Dragon_Idle")))
      (:then_3
        ;[1 1 1] BeginPlay
        (if (and (Variables|Default|GetIsAtBoss) (not (Variables|Default|GetHasRunOnce)))
          (Utilities|FlowControl|Delay (Variables|Default|GetEntranceTime))
          (UserInterface|Viewport|AddtoViewport (stale EventBeginPlay _output_get) 0)
          (Variables|Default|SetHasRunOnce true))))
    (else
      (Development|PrintString "Dead"))))

(fn ConstructionScript)

(fn UpdateHealth
  (bind _healthbar (Variables|Default|GetHealthBar))
  ;[1 1 1] Update Health Bars
  (Variables|/Game/Game/Blueprints/BossHealthBar.BossHealthBar_C|SetHP1 _healthbar (Variables|Default|GetH1%25))
  (Variables|/Game/Game/Blueprints/BossHealthBar.BossHealthBar_C|SetHP2 _healthbar (Variables|Default|GetH2%25))
  (Variables|/Game/Game/Blueprints/BossHealthBar.BossHealthBar_C|SetHP3 _healthbar (Variables|Default|GetH3%25))
  (Variables|/Game/Game/Blueprints/BossHealthBar.BossHealthBar_C|SetHP4 _healthbar (Variables|Default|GetH4%25)))