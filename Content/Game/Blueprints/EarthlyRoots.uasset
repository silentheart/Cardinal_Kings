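; Paper2D root attack that damages the player caught in its zone when a strike is triggered.
; StrikeR shows the DragonRoots flipbook on all root components, arms damage, then after a brief delay reuses the BeginPlay reset to clear both.
; B7 overlap events track whether MyCharacter is in range and store its reference.
; Tick polls both flags, calling DamageSystem on the player and disarming so each strike hits once.
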(event OnComponentBeginOverlap(B7)
  (params (OtherActor :type Actor%20Object%20Reference) (OtherComp :type Primitive%20Component%20Object%20Reference) (OtherBodyIndex :type Integer) (bFromSweep :type Boolean) (SweepResult :type Hit%20Result%20Structure%20%28by%20ref%29))
  ;[1 1 1] Lightning Zones
  (bind _asmy_character (Utilities|Casting|CastToMyCharacter OtherActor))
  (Variables|Default|SetInRangeSeven true)
  (Variables|Default|SetPlayerRef _asmy_character))

(event OnComponentEndOverlap(B7)
  (params (OtherActor :type Actor%20Object%20Reference) (OtherComp :type Primitive%20Component%20Object%20Reference) (OtherBodyIndex :type Integer))
  ;[1 1 1] Lightning Zones
  (Utilities|Casting|CastToMyCharacter OtherActor)
  (Variables|Default|SetInRangeSeven false))

(event Custom|StrikeR
  ;[1 1 1] Strike
  (Variables|Default|SetIsSeven true)
  (Utilities|FlowControl|Sequence
    (:then_0
      (Sprite|SetFlipbook (Variables|Default|GetR1M) "/Game/Game/Textures/Roots/DragonRoots.DragonRoots"))
    (:then_1
      (Sprite|SetFlipbook (Variables|Default|GetR3-R) "/Game/Game/Textures/Roots/DragonRoots.DragonRoots")
      (Sprite|SetFlipbook (Variables|Default|GetR3-L) "/Game/Game/Textures/Roots/DragonRoots.DragonRoots"))
    (:then_2
      (Sprite|SetFlipbook (Variables|Default|GetR5-R) "/Game/Game/Textures/Roots/DragonRoots.DragonRoots")
      (Sprite|SetFlipbook (Variables|Default|GetR5-L) "/Game/Game/Textures/Roots/DragonRoots.DragonRoots"))
    (:then_3
      (Sprite|SetFlipbook (Variables|Default|GetR7-R) "/Game/Game/Textures/Roots/DragonRoots.DragonRoots")
      (Sprite|SetFlipbook (Variables|Default|GetR7-L) "/Game/Game/Textures/Roots/DragonRoots.DragonRoots"))
    (:then_4
      (Sprite|SetFlipbook (Variables|Default|GetR1L) "/Game/Game/Textures/Roots/DragonRoots.DragonRoots")
      (Sprite|SetFlipbook (Variables|Default|GetR1R) "/Game/Game/Textures/Roots/DragonRoots.DragonRoots"))
    (:then_5
      (Sprite|SetFlipbook (Variables|Default|GetR1LL) "/Game/Game/Textures/Roots/DragonRoots.DragonRoots")
      (Sprite|SetFlipbook (Variables|Default|GetR1RR) "/Game/Game/Textures/Roots/DragonRoots.DragonRoots"))
    (:then_6
      (Utilities|FlowControl|Delay (/ 1.0 3.0))
      (Utilities|FlowControl|Sequence
        (:then_0
          (Sprite|SetFlipbook (Variables|Default|GetR1M)))
        (:then_1
          (Sprite|SetFlipbook (Variables|Default|GetR3-R))
          (Sprite|SetFlipbook (Variables|Default|GetR3-L)))
        (:then_2
          (Sprite|SetFlipbook (Variables|Default|GetR5-R))
          (Sprite|SetFlipbook (Variables|Default|GetR5-L)))
        (:then_3
          (Sprite|SetFlipbook (Variables|Default|GetR7-R))
          (Sprite|SetFlipbook (Variables|Default|GetR7-L)))
        (:then_4
          (Sprite|SetFlipbook (Variables|Default|GetR1L))
          (Sprite|SetFlipbook (Variables|Default|GetR1R)))
        (:then_5
          (Sprite|SetFlipbook (Variables|Default|GetR1LL))
          (Sprite|SetFlipbook (Variables|Default|GetR1RR)))
        (:then_6
          (Variables|Default|SetIsSeven false))))))

(event EventBeginPlay
  ;[1 1 1] Strike
  (Utilities|FlowControl|Sequence
    (:then_0
      (Sprite|SetFlipbook (Variables|Default|GetR1M)))
    (:then_1
      (Sprite|SetFlipbook (Variables|Default|GetR3-R))
      (Sprite|SetFlipbook (Variables|Default|GetR3-L)))
    (:then_2
      (Sprite|SetFlipbook (Variables|Default|GetR5-R))
      (Sprite|SetFlipbook (Variables|Default|GetR5-L)))
    (:then_3
      (Sprite|SetFlipbook (Variables|Default|GetR7-R))
      (Sprite|SetFlipbook (Variables|Default|GetR7-L)))
    (:then_4
      (Sprite|SetFlipbook (Variables|Default|GetR1L))
      (Sprite|SetFlipbook (Variables|Default|GetR1R)))
    (:then_5
      (Sprite|SetFlipbook (Variables|Default|GetR1LL))
      (Sprite|SetFlipbook (Variables|Default|GetR1RR)))
    (:then_6
      (Variables|Default|SetIsSeven false))))

(event EventTick
  (params (DeltaSeconds :type Float%20%28single-precision%29))
  ;[1 1 1] DealDamage
  (if (and (Variables|Default|GetIsSeven) (Variables|Default|GetInRangeSeven))
    (Default|DamageSystem (Variables|Default|GetPlayerRef) (Variables|Default|GetPlayerDamage))
    (Variables|Default|SetIsSeven false)))

(fn ConstructionScript)