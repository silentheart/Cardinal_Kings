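; Dragon boss enemy that damages MyCharacter on contact with its box and loses fixed health per DamageEnemy call until destroyed.
; DamageEnemy also spawns an animated floating widget showing its health.
; BeginPlay collects two indexed Waypoints and starts a move to the first, while any actor overlap starts an endless MoveComponentTo loop between two target points.
; An AI left/right patrol and its ChangeDirection call are left unwired.
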(event OnComponentBeginOverlap(Box)
  (params (OtherActor :type Actor%20Object%20Reference) (OtherComp :type Primitive%20Component%20Object%20Reference) (OtherBodyIndex :type Integer) (bFromSweep :type Boolean) (SweepResult :type Hit%20Result%20Structure%20%28by%20ref%29))
  (bind _asmy_character (Utilities|Casting|CastToMyCharacter OtherActor))
  (Default|DamageSystem _asmy_character (Variables|Default|GetDamage%20Val)))

(event Custom|DamageEnemy
  ;[1 1 1] Deals damage to the enemy.
  (Utilities|FlowControl|Sequence
    (:then_0
      (bind _returnvalue (UserInterface|CreateWidget "/Game/Game/Blueprints/FloatingText_Widget.FloatingText_Widget_C" 0 self))
      (Utilities|FlowControl|Delay 0.2)
      (Variables|/Game/Game/Blueprints/FloatingText_Widget.FloatingText_Widget_C|SetFloat%20Damage _returnvalue (Math|Conversions|ToFloat(Integer) (Variables|Default|GetEnemy%20Health)))
      (UserInterface|Viewport|AddtoViewport _returnvalue 0)
      (UserInterface|Animation|PlayAnimation _returnvalue (Variables|/Game/Game/Blueprints/FloatingText_Widget.FloatingText_Widget_C|GetFloating%20Text%20ani _returnvalue) 0.0 1 "Forward"))
    (:then_1
      (bind _output_get (Variables|Default|SetEnemy%20Health (- (Variables|Default|GetEnemy%20Health) 34)))
      (if (<= _output_get 0)
        (Actor|DestroyActor)))))

(event Custom|MoveToPoint
  (bind _returnvalue (AI|GetAIController self))
  (AI|Navigation|SimpleMovetoLocation _returnvalue (Variables|Default|GetTargetLocation)))

(event Custom|ChangeDirection
  (bind _waypoints (Variables|Default|GetWaypoints))
  (bind _item (Utilities|Array|Get(acopy) _waypoints))
  (bind _returnvalue (Transformation|GetActorLocation _item))
  (if (Math|Vector|Equal(Vector) (Variables|Default|GetTargetLocation) _returnvalue 0.0001)
    (Variables|Default|SetTargetLocation (Transformation|GetActorLocation (Utilities|Array|Get(acopy) _waypoints 1)))
    (else
      (Variables|Default|SetTargetLocation _returnvalue))))

(event Game|Damage|EventAnyDamage
  (params (Damage :type Float%20%28single-precision%29) (DamageType :type Damage%20Type%20Object%20Reference) (InstigatedBy :type Controller%20Object%20Reference) (DamageCauser :type Actor%20Object%20Reference)))

(event EventBeginPlay
  (bind _outactors (Actor|GetAllActorsOfClass "/Game/Game/Blueprints/Waypoint.Waypoint_C"))
  (for _array_element _outactors
    (Math|Integer|CompareInt (Variables|/Game/Game/Blueprints/Waypoint.Waypoint_C|Getindex _array_element) (Variables|Default|GetWaypoint1)
      (:>
        (Math|Integer|CompareInt (Variables|/Game/Game/Blueprints/Waypoint.Waypoint_C|Getindex _array_element) (Variables|Default|GetWaypoint2) :!label _label
          (:==
            (Utilities|Array|Add (Variables|Default|GetWaypoints) _array_element))))
      (:==
        (Utilities|Array|Add (Variables|Default|GetWaypoints) _array_element)
        (Variables|Default|SetTargetLocation (Transformation|GetActorLocation _array_element)))
      (:<
        (goto _label))))
  (AI|Navigation|SimpleMovetoLocation (stale Custom|MoveToPoint _returnvalue) (Variables|Default|GetTargetLocation)))

(event EventTick
  (params (DeltaSeconds :type Float%20%28single-precision%29)))

(event Collision|EventActorBeginOverlap
  (params (OtherActor :type Actor%20Object%20Reference))
  (bind _returnvalue (VehicleSound|GetRootComponent))
  (Components|MoveComponentTo _returnvalue (Transformation|GetActorLocation (Variables|Default|Gettargetpoint)) "0, 0,0.000000" true true 5.0 :!label _label)
  (Utilities|FlowControl|Delay 1.0)
  (Components|MoveComponentTo _returnvalue (Transformation|GetActorLocation (Variables|Default|Gettargetpoint2)) "0, 0, 0" true true 5.0)
  (goto _label))

(fn ConstructionScript)